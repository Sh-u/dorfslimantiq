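; BP_TileStack is an actor that holds a randomized stack of tile types for the game.
; On BeginPlay it casts and stores the first player controller as BP_PlayerController, then fills the stack with an initial batch of tiles.
; AddTilesToStack appends random tile types to AvailableTiles by converting random integers to the E_TileTypes enum.
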(event EventBeginPlay
  (bind _asbp_player_controller (Utilities|Casting|CastToBP_PlayerController (Game|GetPlayerController 0)))
  (Variables|Default|Setplayer_controller _asbp_player_controller)
  (CallFunction|AddTilestoStack 10))

(event Collision|EventActorBeginOverlap
  (params (OtherActor :type Actor%20Object%20Reference)))

(event EventTick
  (params (DeltaSeconds :type Float%20%28single-precision%29)))

(fn ConstructionScript)

(fn AddTilestoStack
  (params (amount :type Integer))
  (for _index (range 1 amount)
    (Utilities|Array|Add (Variables|Default|Getavailable_tiles) (Utilities|Enum|ByteToEnumE_TileTypes (Math|Conversions|ToByte(Integer) (Math|Random|RandomIntegerinRange 1 5))))))