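; Player controller for a hex tile-placement game, handling the HUD, tile stack, camera and score-driven progression.
; It spawns the next stack tile, rotates it in 60-degree steps and broadcasts ReplaceTile when a ghost tile is clicked.
; Reaching the score threshold triggers level-up, adding tiles, spawning bundle choices and doubling the threshold.
; Tick pans the camera within hex-grid bounds, refreshed on placement, with speed and arm length interpolated from wheel zoom.
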(event Custom|Extend%20map
  (params (spawn_location :type Vector) (target_tile :type BP%20Tile%20Object%20Reference) (score_to_add :type Integer))
  (bind _hexgrid (Variables|Default|Gethexgrid))
  (bind _boxextent (Collision|GetActorBounds _hexgrid false true))
  (CallFunction|SetMapSize (.x _boxextent) (.y _boxextent)))

(event Custom|onLevelUp
  (Default|AddTilestoStack (Variables|Default|Gettile_stack) 5)
  (bind _availablebundles (CallFunction|GetAvailableBundles))
  (bind _result (Utilities|Set|ToArray _availablebundles))
  (CallFunction|SpawnBundles _result)
  (Variables|Default|Setthreshold (* (Variables|Default|Getthreshold) 2))
  (Variables|Default|Setlevel (+ (Variables|Default|Getlevel) 1))
  (Default|CallPickBundle))

(event Custom|onPickItemFromStack
  (bind _tile_stack (Variables|Default|Gettile_stack))
  (bind _available_tiles (Variables|/Game/Project/Blueprints/BP_TileStack.BP_TileStack_C|Getavailable_tiles _tile_stack))
  (if (> (Utilities|Array|Length _available_tiles) 0)
    (Variables|Default|Setselected_tile (Utilities|Array|Get(acopy) _available_tiles))
    (Utilities|Array|RemoveIndex _available_tiles)
    (Class|PanelWidget|RemoveChildat (Variables|/Game/Project/Blueprints/BP_UI.BP_UI_C|Gettile_stack_box (Variables|Default|GetUI)))
    (bind _returnvalue (Game|SpawnActorfromClass "/Game/Project/Blueprints/BP_Tile.BP_Tile_C" (Math|Transform|MakeTransform "0.000000,800.000000,0.000000" "0, 0, 0" "1.000000,1.000000,1.000000") "Undefined" 0 (Variables|Default|Getselected_tile) 0))
    (Variables|Default|Setselected_tile_actor _returnvalue)
    (else
      (Variables|Default|Setselected_tile_actor 0)
      (Variables|Default|Setselected_tile "NewEnumerator0")
      (Widget|RemovefromParent (Variables|Default|Getscore_text_popup)))))

(event EventBeginPlay
  (bind _returnvalue (UserInterface|CreateWidget "/Game/Project/Blueprints/BP_ScorePopup.BP_ScorePopup_C"))
  (UserInterface|Viewport|AddtoViewport _returnvalue 0)
  (Widget|SetVisibility _returnvalue "Collapsed")
  (Variables|Default|Setscore_text_popup _returnvalue)
  (Default|CallCreatedScorePopupWidget)
  (bind _returnvalue_2 (UserInterface|CreateWidget "/Game/Project/Blueprints/BP_UI.BP_UI_C"))
  (Variables|Default|SetUI _returnvalue_2)
  (UserInterface|Viewport|AddtoViewport _returnvalue_2 0)
  (EventDispatchers|BindEventtoLevelUp (delegate Custom|onLevelUp))
  (Variables|Default|Setcamera_pawn (Game|Player|GetPlayerPawn 0))
  (bind _returnvalue_3 (Actor|GetActorOfClass "/Game/Project/Blueprints/BP_HexGrid.BP_HexGrid_C"))
  (bind _output_get (Variables|Default|Sethexgrid _returnvalue_3))
  (CallFunction|SetMapSize (.x (.BoxExtent (Collision|GetActorBounds _output_get false true))) (.y (.BoxExtent (Collision|GetActorBounds _output_get false true))))
  (Input|SetInputModeGameandUI self 0 "LockAlways" false false)
  (EventDispatchers|BindEventtoReplaceTile self (delegate Custom|Extend%20map))
  (bind _returnvalue_4 (Actor|GetActorOfClass "/Game/Project/Blueprints/BP_TileStack.BP_TileStack_C"))
  (Variables|Default|Settile_stack _returnvalue_4)
  (EventDispatchers|BindEventtoPickItemfromStack (delegate Custom|onPickItemFromStack))
  (Default|CallPickItemfromStack))

(event EventTick
  (params (DeltaSeconds :type Float%20%28single-precision%29))
  (CallFunction|MoveCamera))

(event Input|ActionEvents|InputActionAction
  (params (Key :type Key%20Structure :default "None"))
  (bind _returnvalue (Viewport|GetViewportSize))
  (:Pressed
    (Development|PrintString (Utilities|String|ToString(Vector2d) (Viewport|GetViewportSize)))
    (bind _returnvalue_2 (Class|WidgetLayoutLibrary|GetMousePositiononViewport))
    (Development|PrintString (Class|KismetStringLibrary|BuildStringVector2d "" "viewport pos: " _returnvalue_2))
    (Development|PrintString (Class|KismetStringLibrary|BuildStringDouble "" "Mouse x:" (Variables|Default|Getmouse_x)))
    (Development|PrintString (Class|KismetStringLibrary|BuildStringDouble "" "normalized: " (Math|Float|Clamp(Float) (Math|Float|NormalizetoRange (Variables|Default|Getmouse_x) (* (* (.x _returnvalue) 0.9) 2.0) (* (.x _returnvalue) 2.0)))))))

(event Input|ActionEvents|InputActionRight
  (params (Key :type Key%20Structure :default "None"))
  (:Pressed
    (Variables|Default|Setcamera_movement (+ (Variables|Default|Getcamera_movement) "0.000000,1.000000,0.000000")))
  (:Released
    (Variables|Default|Setcamera_movement (- (Variables|Default|Getcamera_movement) "0.000000,1.000000,0.000000"))))

(event Input|ActionEvents|InputActionUp
  (params (Key :type Key%20Structure :default "None"))
  (:Pressed
    (Variables|Default|Setcamera_movement (+ (Variables|Default|Getcamera_movement) "1.000000,0.000000,0.000000")))
  (:Released
    (Variables|Default|Setcamera_movement (- (Variables|Default|Getcamera_movement) "1.000000,0.000000,0.000000"))))

(event Input|ActionEvents|InputActionDown
  (params (Key :type Key%20Structure :default "None"))
  (:Pressed
    (Variables|Default|Setcamera_movement (- (Variables|Default|Getcamera_movement) "1.000000,0.000000,0.000000")))
  (:Released
    (Variables|Default|Setcamera_movement (+ (Variables|Default|Getcamera_movement) "1.000000,0.000000,0.000000"))))

(event Input|ActionEvents|InputActionLeft
  (params (Key :type Key%20Structure :default "None"))
  (:Pressed
    (Variables|Default|Setcamera_movement (- (Variables|Default|Getcamera_movement) "0.000000,1.000000,0.000000")))
  (:Released
    (Variables|Default|Setcamera_movement (+ (Variables|Default|Getcamera_movement) "0.000000,1.000000,0.000000"))))

(event Input|ActionEvents|InputActionRotate
  (params (Key :type Key%20Structure :default "None"))
  (bind _selected_tile_actor (Variables|Default|Getselected_tile_actor))
  (:Pressed
    (Utilities|IsValid _selected_tile_actor
      (:Is%20Valid
        (Transformation|SetActorRotation (Variables|Default|Getselected_tile_actor) (Math|Rotator|MakeRotator 0.0 0.0 (+ (.yaw (Transformation|GetActorRotation _selected_tile_actor)) 6e+01)))
        (Default|CallRotateTile)))))

(event Input|MouseEvents|MouseWheelUp
  (params (Key :type Key%20Structure :default "None"))
  (:Pressed
    (Variables|Default|Setcamera_zoom (Math|Float|Clamp(Float) (+ (Variables|Default|Getcamera_zoom) 0.1) 0.1))))

(event Input|MouseEvents|MouseWheelDown
  (params (Key :type Key%20Structure :default "None"))
  (:Pressed
    (Variables|Default|Setcamera_zoom (Math|Float|Clamp(Float) (- (Variables|Default|Getcamera_zoom) 0.1) 0.1))))

(event Input|MouseEvents|LeftMouseButton
  (params (Key :type Key%20Structure :default "None"))
  (bind _returnvalue (Game|GetPlayerController 0))
  (bind (_hitresult _returnvalue_2) (Game|Player|GetHitResultUnderCursorbyChannel _returnvalue "TraceTypeQuery1" true))
  (bind _hitactor (Collision|BreakHitResult _hitresult))
  (:Pressed
    (if (not (Variables|Default|Getdisable_raycasting))
      (if _returnvalue_2
        (Utilities|IsValid _hitactor
          (:Is%20Valid
            (bind _asbp_ghost_tile (Utilities|Casting|CastToBP_GhostTile _hitactor)
              (:then
                (if (Utilities|IsValid (Variables|Default|Getselected_tile_actor))
                  (Development|PrintString (Utilities|String|BuildString(Integer) "" "Items amount: " (Utilities|Array|Length (Variables|/Game/Project/Blueprints/BP_TileStack.BP_TileStack_C|Getavailable_tiles (Variables|Default|Gettile_stack)))))
                  (Default|CallReplaceTile (Transformation|GetActorLocation _hitactor) (Variables|Default|Getselected_tile_actor) (Variables|/Game/Project/Blueprints/BP_GhostTile.BP_GhostTile_C|Getcalculated_score _asbp_ghost_tile))
                  (Actor|DestroyActor _asbp_ghost_tile)))
              (:CastFailed
                (Development|PrintString "Failed to cast to ghostTile"))))
          (:Is%20Not%20Valid
            (Development|PrintString "Not valid hit")))))))

(event Input|KeyboardEvents|B
  (params (Key :type Key%20Structure :default "None"))
  (:Pressed
    (Widget|SetVisibility (Variables|/Game/Project/Blueprints/BP_UI.BP_UI_C|Getselected_item_button (Variables|Default|GetUI)) "Visible")
    (Variables|Default|Setselected_tile "NewEnumerator0")))

(fn ConstructionScript)

(fn MoveCamera
  (bind _returnvalue (Class|WidgetLayoutLibrary|GetViewportScale))
  (bind _camera_movement (Variables|Default|Getcamera_movement))
  (bind _min_camera_speed (Variables|Default|Getmin_camera_speed))
  (bind _max_camera_speed (Variables|Default|Getmax_camera_speed))
  (bind _camera_zoom (Variables|Default|Getcamera_zoom))
  (bind _camera_pawn (Variables|Default|Getcamera_pawn))
  (bind _grid_x_size (Variables|Default|Getgrid_x_size))
  (bind _grid_y_size (Variables|Default|Getgrid_y_size))
  (bind _returnvalue_2 (Math|Float|Lerp _max_camera_speed _min_camera_speed _camera_zoom))
  (bind _returnvalue_3 (Math|Vector|Normalize _camera_movement))
  (bind _returnvalue_4 (Transformation|GetActorLocation _camera_pawn))
  (bind _returnvalue_5 (+ _returnvalue_3 "" "" "" ""))
  (bind _returnvalue_6 (Math|Vector|Normalize _returnvalue_5))
  (bind _returnvalue_7 (* _returnvalue_6 _returnvalue_2))
  (bind _returnvalue_8 (+ _returnvalue_7 _returnvalue_4))
  (bind _returnvalue_9 (Class|WidgetLayoutLibrary|GetMousePositiononViewport))
  (Variables|Default|Setmouse_x (* _returnvalue (.x _returnvalue_9)))
  (Variables|Default|Setmouse_y (* _returnvalue (.y _returnvalue_9)))
  (Transformation|SetActorLocationAndRotation _camera_pawn (Math|Vector|MakeVector (Math|Float|Clamp(Float) (.x _returnvalue_8) (* _grid_x_size -1.0) _grid_x_size) (Math|Float|Clamp(Float) (.y _returnvalue_8) (* _grid_y_size -1.0) _grid_y_size) 2e+02))
  (bind _asbp_camera_pawn (Utilities|Casting|CastToBP_CameraPawn (Variables|Default|Getcamera_pawn)))
  (Variables|/Script/Engine.SpringArmComponent|SetTargetArmLength (Variables|/Game/Project/Blueprints/BP_CameraPawn.BP_CameraPawn_C|GetSpringArm _asbp_camera_pawn) (Math|Float|Lerp (Variables|Default|Getmin_zoom_distance) (Variables|Default|Getmax_zoom_distance) (Variables|Default|Getcamera_zoom))))

(fn SetMapSize
  (params (box_extent_x :type Float%20%28double-precision%29) (box_extent_y :type Float%20%28double-precision%29))
  (Variables|Default|Setgrid_x_size (* box_extent_x 1.5))
  (Variables|Default|Setgrid_y_size (* box_extent_y 1.5)))

(fn AddCardtoInventory
  (params (picked_bundle :type BP%20Bundle%20Object%20Reference))
  (for _array_element (Variables|/Game/Project/Blueprints/BP_Bundle.BP_Bundle_C|Gettiles picked_bundle)
    (Utilities|Array|Add (Variables|Default|Getinventory) _array_element))
  (for _array_element_2 (Variables|Default|Getspawned_bundles)
    (Actor|DestroyActor _array_element_2)))

(fn GetAvailableBundles
  (bind _bundle_types (Variables|Default|Getbundle_types))
  (if (< (Variables|Default|Getlevel) 5)
    (return (Utilities|Select :Index "NewEnumerator0" :NewEnumerator0 _bundle_types :NewEnumerator1 _bundle_types))))

(fn AddScore
  (params (score_to_add :type Integer))
  (bind _output_get (Variables|Default|Setscore (+ (Variables|Default|Getscore) score_to_add)))
  (if (>= _output_get (Variables|Default|Getthreshold))
    (Default|CallLevelUp)))

(fn SpawnBundles
  (params (bundles_to_spawn :type Array%20of%20BP_Bundles%20Enums :default "NewEnumerator0"))
  (for _array_element bundles_to_spawn
    (bind _returnvalue (Game|SpawnActorfromClass "/Game/Project/Blueprints/BP_Bundle.BP_Bundle_C" (Math|Transform|MakeTransform "0, 0, 0" "0, 0, 0" "1.000000,1.000000,1.000000") "Undefined" 0 _array_element 0))
    (Utilities|Array|Add (Variables|Default|Getspawned_bundles) _returnvalue)))