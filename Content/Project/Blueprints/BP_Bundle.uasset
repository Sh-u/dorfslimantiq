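; BP_Bundle is a bundle of tile types, themed by its BundleType as either Nature or Buildings.
; On BeginPlay it fills its Tiles array with a small randomized number of entries.
; Nature bundles pick randomly between two tile types per entry, while Buildings bundles always add the same type, as their random switch has only one possible value.
; It contains no other active logic.
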(event EventBeginPlay
  (switch Utilities|FlowControl|Switch|SwitchonBP_Bundles (Variables|Default|Getbundle_type)
    (:NewEnumerator0
      (for _index (range 0 (Math|Random|RandomIntegerinRange 2 3))
        (switch int (Math|Random|RandomIntegerinRange 0 1)
          (:0
            (Variables|Default|Settile_type "NewEnumerator5"))
          (:1
            (Variables|Default|Settile_type "NewEnumerator3")))
        (Utilities|Array|Add (Variables|Default|Gettiles) (Variables|Default|Gettile_type))))
    (:NewEnumerator1
      (for _index_2 (range 0 (Math|Random|RandomIntegerinRange 2 3))
        (switch int (Math|Random|RandomIntegerinRange 0 0)
          (:0
            (Variables|Default|Settile_type "NewEnumerator2")
            (Utilities|Array|Add (Variables|Default|Gettiles) (Variables|Default|Gettile_type))))))))

(event Collision|EventActorBeginOverlap
  (params (OtherActor :type Actor%20Object%20Reference)))

(event EventTick
  (params (DeltaSeconds :type Float%20%28single-precision%29)))

(fn ConstructionScript)