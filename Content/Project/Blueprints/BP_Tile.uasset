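; BP_Tile is a tile actor that takes on one of five terrain types: meadow, buildings, river, mountains or forest.
; On BeginPlay it switches on TileType and adds a child actor component of the matching terrain Blueprint.
; CreateSocketLocations caches the world positions of the static mesh's sockets.
; GetAvailableSpawnLocations line-traces from the mesh to each cached position and returns those with no hit as open spawn points.
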(event EventBeginPlay
  (Variables|Default|Setstatic_mesh (Variables|Default|GetStaticMesh))
  (switch Utilities|FlowControl|Switch|SwitchonBP_TileTypes (Variables|Default|Gettile_type)
    (:NewEnumerator1
      (bind _returnvalue (AddComponent|AddChildActorComponent false))
      (ChildActorComponent|SetChildActorClass _returnvalue "/Game/Project/Blueprints/BP_Meadow.BP_Meadow_C"))
    (:NewEnumerator2
      (bind _returnvalue_2 (AddComponent|AddChildActorComponent false))
      (ChildActorComponent|SetChildActorClass _returnvalue_2 "/Game/Project/Blueprints/TileTypes/BP_Buildings.BP_Buildings_C"))
    (:NewEnumerator3
      (bind _returnvalue_3 (AddComponent|AddChildActorComponent false))
      (ChildActorComponent|SetChildActorClass _returnvalue_3 "/Game/Project/Blueprints/BP_River.BP_River_C"))
    (:NewEnumerator4
      (bind _returnvalue_4 (AddComponent|AddChildActorComponent false))
      (ChildActorComponent|SetChildActorClass _returnvalue_4 "/Game/Project/Blueprints/BP_Mountains.BP_Mountains_C"))
    (:NewEnumerator5
      (bind _returnvalue_5 (AddComponent|AddChildActorComponent false))
      (ChildActorComponent|SetChildActorClass _returnvalue_5 "/Game/Project/Blueprints/BP_Forest.BP_Forest_C"))))

(event Collision|EventActorBeginOverlap
  (params (OtherActor :type Actor%20Object%20Reference)))

(event EventTick
  (params (DeltaSeconds :type Float%20%28single-precision%29)))

(fn ConstructionScript)

(fn GetAvailableSpawnLocations
  (for _array_element (Variables|Default|Getsocket_locations)
    (bind _returnvalue (Collision|LineTraceByChannel (Transformation|GetWorldLocation (Variables|Default|GetStaticMesh)) _array_element "TraceTypeQuery1" false 0 "None"))
    (if (not _returnvalue)
      (Utilities|Array|Add (LocalVariables|Getavailable_locations) _array_element)))
  (return (LocalVariables|Getavailable_locations)))

(fn CreateSocketLocations
  (for _array_element (Transformation|GetAllSocketNames (Variables|Default|GetStaticMesh))
    (Utilities|Array|Add (Variables|Default|Getsocket_locations) (Transformation|GetSocketLocation (Variables|Default|GetStaticMesh) _array_element))))