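; Ghost placeholder tile that previews the player's selected tile and its potential score while the cursor hovers over it.
; Hover copies the selected tile's material and child actor, binds 60-degree rotation to the player controller, and shows a score popup.
; Line traces to socket locations double the base score for each same-type neighboring tile.
; Cursor exit restores the material and rotation, destroys child actors, unbinds rotation and hides the popup.
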(event Custom|OnBeginCursorOver_Event
  (params (TouchedActor :type Actor%20Object%20Reference))
  (if (Utilities|Enum|Equal(Enum) (Variables|/Script/dorfslimantiq.PC|GetSelected_Tile_Type (Variables|Default|Getplayer_controller)) "Empty")
    (Development|PrintString "No tile selected")
    (else
      (EventDispatchers|BindEventtoRotateTile (Variables|Default|Getplayer_controller) (delegate Custom|onRotateTile))
      (bind _asbp_tile (Utilities|Casting|CastToBP_Tile (Variables|/Script/dorfslimantiq.PC|GetSelected_Tile_Actor (Variables|Default|Getplayer_controller))))
      (Variables|Default|Setselected_tile _asbp_tile)
      (Rendering|Material|SetMaterial (Variables|Default|GetStaticMesh) 0 (Rendering|Material|GetMaterial (Variables|/Game/Project/Blueprints/BP_Tile.BP_Tile_C|GetStaticMesh (Variables|Default|Getselected_tile)) 0))
      (bind _returnvalue (AddComponent|AddChildActorComponent false (Math|Transform|MakeTransform "0, 0, 0" (Transformation|GetActorRotation (Variables|Default|Getselected_tile)) "1.000000,1.000000,1.000000")))
      (ChildActorComponent|SetChildActorClass _returnvalue (Utilities|GetClass (Utilities|Array|Get(acopy) (Actor|GetAllChildActors (Variables|Default|Getselected_tile) true))))
      (Utilities|IsValid (Variables|Default|Getscore_popup_widget)
        (:Is%20Valid
          (Widget|SetVisibility (Variables|Default|Getscore_popup_widget) "HitTestInvisible")
          (Variables|/Game/Project/Blueprints/Widgets/WBP_ScorePopup.WBP_ScorePopup_C|Settile_location (Variables|Default|Getscore_popup_widget) (Transformation|GetActorLocation self))
          (bind _base_score (CallFunction|GetBaseTileScore (Variables|/Script/dorfslimantiq.PC|GetSelected_Tile_Type (Variables|Default|Getplayer_controller))))
          (bind _output_get (Variables|Default|Setcalculated_score _base_score))
          (for _array_element (Variables|Default|Getsocket_locations self)
            (bind (_outhit _returnvalue_2) (Collision|LineTraceByChannel (Transformation|GetActorLocation self) _array_element "TraceTypeQuery1" false 0 "None" true "(R=1.000000,G=0.000000,B=0.000000,A=1.000000)" "(R=0.000000,G=1.000000,B=0.000000,A=1.000000)" 1.0))
            (if _returnvalue_2
              (if (not (== (Utilities|GetClass (.HitActor (Collision|BreakHitResult _outhit))) "BP_GhostTile_C"))
                (bind _asbp_tile_2 (Utilities|Casting|CastToBP_Tile (.HitActor (Collision|BreakHitResult _outhit))))
                (if (Utilities|Enum|Equal(Enum) (Variables|/Game/Project/Blueprints/BP_Tile.BP_Tile_C|Gettile_type _asbp_tile_2) (Variables|/Script/dorfslimantiq.PC|GetSelected_Tile_Type (Variables|Default|Getplayer_controller)))
                  (Development|PrintString "hit same")
                  (Variables|Default|Setcalculated_score (+ (Variables|Default|Getcalculated_score) _output_get))))))
          (Rendering|Components|TextRender|SetText (Variables|/Game/Project/Blueprints/Widgets/WBP_ScorePopup.WBP_ScorePopup_C|Getscore_popup_text (Variables|Default|Getscore_popup_widget)) (Utilities|Text|ToText(String) (Utilities|String|BuildString(Integer) "" "+" (Variables|Default|Getcalculated_score)))))
        (:Is%20Not%20Valid
          (Development|PrintString "invalid widget"))))))

(event Custom|OnEndCursorOver_Event
  (params (TouchedActor :type Actor%20Object%20Reference))
  (EventDispatchers|UnbindallEventsfromRotateTile (Variables|Default|Getplayer_controller))
  (Variables|Default|Setcalculated_score 0)
  (Transformation|SetActorRotation self)
  (Rendering|Material|SetMaterial (Variables|Default|GetStaticMesh) 0 (Variables|Default|Getold_material))
  (Variables|Default|Setselected_tile 0)
  (for _array_element (Actor|GetAllChildActors self true)
    (Actor|DestroyActor _array_element)
    (Utilities|IsValid (Variables|Default|Getscore_popup_widget)
      (:Is%20Valid
        (Widget|SetVisibility (Variables|Default|Getscore_popup_widget) "Collapsed")))))

(event Custom|onCreatedScorePopupWidget
  (Variables|Default|Setscore_popup_widget (Variables|/Game/Project/Blueprints/BP_PlayerController.BP_PlayerController_C|Getscore_text_popup (Variables|Default|Getplayer_controller))))

(event Custom|onRotateTile
  (Transformation|SetActorRotation self (Math|Rotator|MakeRotator 0.0 0.0 (+ (.yaw (Transformation|GetActorRotation self)) 6e+01))))

(event EventBeginPlay
  (bind _asbp_player_controller (Utilities|Casting|CastToBP_PlayerController (Game|GetPlayerController 0)))
  (bind _output_get (Variables|Default|Setplayer_controller _asbp_player_controller))
  (Utilities|IsValid _output_get
    (:Is%20Valid
      (Utilities|IsValid (Variables|/Game/Project/Blueprints/BP_PlayerController.BP_PlayerController_C|Getscore_text_popup (Variables|Default|Getplayer_controller))
        (:Is%20Valid
          (Variables|Default|Setscore_popup_widget (Variables|/Game/Project/Blueprints/BP_PlayerController.BP_PlayerController_C|Getscore_text_popup (Variables|Default|Getplayer_controller))))
        (:Is%20Not%20Valid
          (EventDispatchers|BindEventtoCreatedScorePopupWidget (Variables|Default|Getplayer_controller) (delegate Custom|onCreatedScorePopupWidget))))
      (bind _output_get_2 (Variables|Default|Setold_static_mesh (Variables|Default|GetStaticMesh)))
      (bind _returnvalue (Rendering|Material|GetBaseMaterial (Rendering|Material|GetMaterial _output_get_2 0)))
      (Variables|Default|Setold_material _returnvalue)
      (Default|CreateSocketLocations self)
      (EventDispatchers|BindEventtoOnBeginCursorOver (delegate Custom|OnBeginCursorOver_Event))
      (EventDispatchers|AssignOnEndCursorOver (delegate Custom|OnEndCursorOver_Event)))
    (:Is%20Not%20Valid
      (Development|PrintString "Player  controller is not valid"))))

(event EventTick
  (params (DeltaSeconds :type Float%20%28single-precision%29)))

(event Collision|EventActorBeginOverlap
  (params (OtherActor :type Actor%20Object%20Reference)))

(fn ConstructionScript)

(fn GetBaseTileScore
  (params (selected_tile :type ETiletype%20Enum :default "Empty"))
  (if (Utilities|Enum|Equal(Enum) selected_tile "Empty")
    (return 0)
    (else
      (return 10))))