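; BP_HexGrid is a grid actor for tile placement that destroys its Sphere component and binds a tile-replace handler at BeginPlay.
; The bound event forwards the selected tile and location to HandleReplaceTIle.
; SpawnGTiles adds BP_GhostTile child actors at given locations.
; Starting-tile construction, tile attachment, ghost spawning from socket locations, and scoring logic are disconnected, and SpawnTile and Tick are empty.
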(event Custom|SpawnTile
  (params (spawn_location :type Vector) (target_tile :type BP%20Tile%20Object%20Reference) (score_to_add :type Integer)))

(event Custom|onTileReplace
  (params (Selected_Tile :type Tile%20Object%20Reference) (Location :type Vector%20%28by%20ref%29)))

(event Custom|CustomEvent
  (params (Selected_Tile :type Tile%20Object%20Reference) (Location :type Vector%20%28by%20ref%29))
  (Class|Hexgrid|HandleReplaceTIle Selected_Tile Location))

(event EventBeginPlay
  (Components|DestroyComponent (Variables|Default|GetSphere))
  (EventDispatchers|BindEventtoOnReplaceTile (delegate Custom|CustomEvent)))

(event EventTick
  (params (DeltaSeconds :type Float%20%28single-precision%29)))

(fn ConstructionScript)

(fn SpawnGTiles
  (params (ghost_tiles_spawn_location :type Array%20of%20Vectors))
  (for _array_element ghost_tiles_spawn_location
    (bind _returnvalue (AddComponent|AddChildActorComponent false (Math|Transform|MakeTransform _array_element "0, 0, 0" "1.000000,1.000000,1.000000")))
    (ChildActorComponent|SetChildActorClass _returnvalue "/Game/Project/Blueprints/BP_GhostTile.BP_GhostTile_C")))